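; Enemy Blueprint that takes damage, shows its health in an on-screen HealthBar widget and triggers the player's win when defeated.
; A GotHit flag, not reset here, filters multiple hits; damage lowers Health and updates the widget.
; A hit arriving with Health already below 1 fires a camera-change dispatcher, sets Win and disables player movement.
; A construction-script dynamic material tints red on damage, restoring its original color after a delay.
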(event EventBeginPlay
  ;[1 1 1] Get the original Material Color
  (Utilities|FlowControl|Sequence
    (:then_0
      (bind _returnvalue (Rendering|Material|GetVectorParameterValue (Variables|Default|GetDynamicMaterial) "Color" :!class /Script/Engine.MaterialInstanceDynamic))
      (bind _output_get (Variables|Default|SetOriginalColor _returnvalue)))
    (:then_1
      ;[1 1 1] Show UI
      (bind _returnvalue_2 (UserInterface|CreateWidget "/Game/UI/HealthBar.HealthBar_C"))
      (bind _output_get_2 (Variables|Default|SetHealthBarUI _returnvalue_2))
      (Variables|/Game/UI/HealthBar.HealthBar_C|SetHealthUI _output_get_2 (Variables|Default|GetHealth))
      (UserInterface|Viewport|AddtoViewport _output_get_2 0))))

(event Game|Damage|EventAnyDamage
  (params (Damage :type Float%20%28single-precision%29) (DamageType :type Damage%20Type%20Object%20Reference) (InstigatedBy :type Controller%20Object%20Reference) (DamageCauser :type Actor%20Object%20Reference))
  (bind _dynamicmaterial (Variables|Default|GetDynamicMaterial))
  ;[1 1 1] Hit Component
  (Utilities|FlowControl|Sequence
    (:then_0
      (if (not (Variables|Default|GetGotHit))
        (Variables|Default|SetGotHit true)
        (if (< (Variables|Default|GetHealth) 1.0)
          (Default|CallChangeCamear) ; Using EventDispatcher to Communicate with other blueprints ( Level blueprint)
          ;[1 1 1] Show Winning Pose and Stop Moving
          (bind _output_get (Variables|Default|Setdead true))
          (bind _asmy_character (Utilities|Casting|CastToMyCharacter (Game|GetPlayerCharacter 0)))
          (Variables|/Game/Blueprint/MyCharacter.MyCharacter_C|Setwin _asmy_character _output_get)
          (Pawn|Components|CharacterMovement|DisableMovement (Variables|/Script/Engine.Character|GetCharacterMovement _asmy_character))
          (else
            (bind _output_get_2 (Variables|Default|SetHealth (- (Variables|Default|GetHealth) Damage)))
            ;[1 1 1] To reflect Health Change on UI
            (Variables|/Game/UI/HealthBar.HealthBar_C|SetHealthUI (Variables|Default|GetHealthBarUI) _output_get_2)))))
    (:then_1
      ;[1 1 1] Change Color when being hit and return to previous state after 1 sec
      (Rendering|Material|SetVectorParameterValue _dynamicmaterial "Color" "(R=0.145833,G=0.000000,B=0.000000,A=1.000000)" :!class /Script/Engine.MaterialInstanceDynamic)
      (Utilities|FlowControl|Delay 1.0)
      (Rendering|Material|SetVectorParameterValue _dynamicmaterial "Color" (stale EventBeginPlay _output_get) :!class /Script/Engine.MaterialInstanceDynamic))))

(fn ConstructionScript
  ;[1 1 1] Creating Dynamic Material to be changed when being hit
  (bind _returnvalue (Rendering|Material|CreateDynamicMaterialInstance (Variables|Character|GetMesh) 0 "/Game/Character/Mannequin/Material/Hit/UE4_maniquen.UE4_maniquen" :!class /Script/Engine.PrimitiveComponent))
  (Variables|Default|SetDynamicMaterial _returnvalue))