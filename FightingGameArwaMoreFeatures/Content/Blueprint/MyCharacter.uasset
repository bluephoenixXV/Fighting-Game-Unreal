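; Player character for a melee fighter that moves along a single world axis, runs while Space is held, and punches or kicks.
; Z and X set Punch and Kick flags, which are never cleared here, and movement input is ignored while Attacking.
; Hand and foot overlap events check their matching flag before applying damage, with kicks hitting harder than punches.
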(event OnComponentBeginOverlap(RightHand)
  (params (OverlappedComponent :type Primitive%20Component%20Object%20Reference) (OtherActor :type Actor%20Object%20Reference) (OtherComp :type Primitive%20Component%20Object%20Reference) (OtherBodyIndex :type Integer) (bFromSweep :type Boolean) (SweepResult :type Hit%20Result%20Structure%20%28by%20ref%29))
  ;[1 1 1] Damage System ( when colliding with right hand)
  (if (Variables|Default|Getpunch)
    (Game|Damage|ApplyDamage OtherActor 1e+01 (Game|GetInstigatorController) self)))

(event OnComponentBeginOverlap(RightFoot)
  (params (OverlappedComponent :type Primitive%20Component%20Object%20Reference) (OtherActor :type Actor%20Object%20Reference) (OtherComp :type Primitive%20Component%20Object%20Reference) (OtherBodyIndex :type Integer) (bFromSweep :type Boolean) (SweepResult :type Hit%20Result%20Structure%20%28by%20ref%29))
  ;[1 1 1] Damage System ( when Colliding with right foot )
  (if (Variables|Default|Getkick)
    (Game|Damage|ApplyDamage OtherActor 2e+01 (Game|GetInstigatorController) self)))

(event EventBeginPlay
  ;[1 1 1] Define Default State ( Palyer Walking and Speed )
  (Variables|/Script/Engine.CharacterMovementComponent|SetMaxWalkSpeed (Variables|Character|GetCharacterMovement) 4.5e+02))

(event Input|AxisEvents|InputAxisX-Axis
  (params (AxisValue :type Float%20%28single-precision%29))
  ;[1 1 1] Side Movement ( while Not Attacking )
  (if (not (Variables|Default|GetAttacking))
    (Pawn|Input|AddMovementInput "0.000000,1.000000, 0" AxisValue false)))

(event Input|KeyboardEvents|SpaceBar
  (params (Key :type Key%20Structure))
  (bind _charactermovement (Variables|Character|GetCharacterMovement))
  ;[1 1 1] Define Running to Walking State ( Player is Running when pressing space bar )
  (:Pressed
    (Variables|/Script/Engine.CharacterMovementComponent|SetMaxWalkSpeed _charactermovement 7e+02))
  (:Released
    (Variables|/Script/Engine.CharacterMovementComponent|SetMaxWalkSpeed _charactermovement 4.5e+02)))

(event Input|KeyboardEvents|Z
  (params (Key :type Key%20Structure))
  ;[1 1 1] Puncning Button
  (:Pressed
    (Variables|Default|Setpunch true)))

(event Input|KeyboardEvents|X
  (params (Key :type Key%20Structure))
  ;[1 1 1] Kicking Button
  (:Pressed
    (Variables|Default|Setkick true)))

(fn ConstructionScript)